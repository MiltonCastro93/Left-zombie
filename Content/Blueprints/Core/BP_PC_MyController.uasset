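; BP_PC_MyController is a player controller that sets up input and the HUD when play begins.
; BeginPlay adds the IMC_Default Enhanced Input mapping context if the subsystem is valid, then calls CreateHUD.
; CreateHUD makes a WB_HUD widget only once, caches it, adds it to the viewport, and switches to game-only input with the mouse cursor hidden.
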(event EventBeginPlay
  (bind _returnvalue (PlayerController|LocalPlayerSubsystems|GetEnhancedInputLocalPlayerSubsystem))
  ;[0 0 0 0.5] Me da Controles sobre el character
  (Utilities|IsValid _returnvalue
    (:Is%20Valid
      (Input|AddMappingContext _returnvalue "/Game/Input/IMC_Default.IMC_Default" 0 "(bIgnoreAllPressedKeysUntilRelease=True,bForceImmediately=False,bNotifyUserSettings=False)")
      ;[0 0 0 0.5] Instancio el HUD
      (CallFunction|CreateHUD))))

(event EventTick
  (params (DeltaSeconds :type Float%20%28single-precision%29)))

(fn ConstructionScript)

(fn CreateHUD
  (bind _returnvalue (Game|GetPlayerController 0))
  (Variables|Default|GetWB_HUD_REF
    (:then)
    (:else
      (bind _returnvalue_2 (UserInterface|CreateWidget "/Game/HUD/WB_HUD.WB_HUD_C" _returnvalue))
      (bind _output_get (Variables|Default|SetWB_HUD_REF _returnvalue_2))
      (UserInterface|Viewport|AddtoViewport _output_get 0)
      (Input|SetInputModeGameOnly _returnvalue false)
      (Variables|Default|SetbShowMouseCursor false))))