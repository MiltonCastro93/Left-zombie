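; Trigger volume actor that turns on a post process effect some time after the player enters it.
; Overlap of the capsule by the player pawn sets an active flag, after which Tick accumulates elapsed time and enables the PostProcess component once the maximum time is reached.
; Nothing clears the flag or disables the effect, and the timer keeps counting after it fires.
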(event OnComponentBeginOverlap(Capsule)
  (params (OverlappedComponent :type Primitive%20Component%20Object%20Reference) (OtherActor :type Actor%20Object%20Reference) (OtherComp :type Primitive%20Component%20Object%20Reference) (OtherBodyIndex :type Integer) (bFromSweep :type Boolean) (SweepResult :type Hit%20Result%20Structure%20%28by%20ref%29))
  (if (== OtherActor (Game|Player|GetPlayerPawn 0))
    (Variables|Default|SetActive true)))

(event EventTick
  (params (DeltaSeconds :type Float%20%28single-precision%29))
  (if (Variables|Default|GetActive)
    (bind _output_get (Variables|Default|SetCurrentTime (+ DeltaSeconds (Variables|Default|GetCurrentTime))))
    (if (>= _output_get (Variables|Default|GetMaxTime))
      (Variables|/Script/Engine.PostProcessComponent|SetbEnabled (Variables|Default|GetPostProcess) true))))

(fn ConstructionScript)